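; BP_BaseSceneProp is a base physics-driven scenery prop that shows a random idle flipbook from four options.
; While nearly stationary, it sets its Box's Y velocity from the scenario impulse held by GM_CtrlAlt24.
; When the main character overlaps it with vertical velocity, it tells the game mode to slow the scenario impulse and boost the character impulse, gated by a short cooldown.
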(event `self.ReceiveBeginPlay`
  (`PaperFlipbookComponent.SetFlipbook` (`self.FB_Prop`) (`KismetArrayLibrary.Array_Random` (`|MakeArray` "/Game/CtrlAltJam/Materials/SceneProps/F1P1/FB_F1P1_Idle.FB_F1P1_Idle" "/Game/CtrlAltJam/Materials/SceneProps/F1P2/FB_F1P2_Idle.FB_F1P2_Idle" "/Game/CtrlAltJam/Materials/SceneProps/F2P1/FB_F2P1_Idle.FB_F2P1_Idle" "/Game/CtrlAltJam/Materials/SceneProps/F2P2/FB_F2P2_Idle.FB_F2P2_Idle" :!type "PaperFlipbook Object Reference")))
  (bind _asgm_ctrl_alt_24 (cast `/Game/CtrlAltJam/Blueprints/Core/GM_CtrlAlt24` (`GameplayStatics.GetGameMode`)))
  (set `self.GameMode` _asgm_ctrl_alt_24))

(event `self.ReceiveTick`
  (params (DeltaSeconds :type "Float (single-precision)"))
  (bind _gamemode (`self.GameMode`))
  (bind _scenarioimpulse (`/Game/CtrlAltJam/Blueprints/Core/GM_CtrlAlt24.ScenarioImpulse` _gamemode))
  (`|ExecutionSequence`
    (:`then_1`
      (if (`KismetMathLibrary.Vector_IsNearlyZero` (`self.GetVelocity`) 0.1)
        (if (not (`KismetMathLibrary.NearlyEqual_FloatFloat` _scenarioimpulse 0.0 0.1))
          (`PrimitiveComponent.SetPhysicsLinearVelocity` (`self.Box`) (`KismetMathLibrary.MakeVector` 0.0 (* _scenarioimpulse (* (`/Game/CtrlAltJam/Blueprints/Core/GM_CtrlAlt24.ScenarioBaseImpulse` _gamemode) 0.4))) false "None"))))))

(event `self.Box.OnComponentBeginOverlap`
  (params (OverlappedComponent :type "PrimitiveComponent Object Reference") (OtherActor :type "Actor Object Reference") (OtherComp :type "PrimitiveComponent Object Reference") (OtherBodyIndex :type Integer) (bFromSweep :type Boolean) (SweepResult :type "HitResult Structure (by ref)"))
  (bind (_returnvalue_x _returnvalue_y _returnvalue_z) (`KismetMathLibrary.BreakVector` (`self.GetVelocity` OtherActor)))
  (if (`GameplayStatics.ObjectIsA` OtherActor "/Game/CtrlAltJam/Blueprints/Core/BP_MainCharacter.BP_MainCharacter_C")
    (if (not (`KismetMathLibrary.NearlyEqual_FloatFloat` _returnvalue_z))
      (`/Engine/EditorBlueprintResources/StandardMacros.DoOnce` false :!label _label
        (:`Completed`
          (`/Game/CtrlAltJam/Blueprints/Core/GM_CtrlAlt24.AddImpulse` (`self.GameMode`) -2.0 15.0)
          (`KismetSystemLibrary.Delay` 1.5)
          (goto _label :!via `Reset`))))))

(fn `UserConstructionScript`)