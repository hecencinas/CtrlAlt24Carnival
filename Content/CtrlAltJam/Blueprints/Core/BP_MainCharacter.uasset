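; BP_MainCharacter is the main character Blueprint, swapping the Du flipbook to match vertical movement.
; It listens to the GM_CtrlAlt24 game mode's impulse event until the first positive character impulse, then flags that it has left the ground and unbinds.
; From then on, Tick picks idle, jump or fly from Z velocity (near zero, rising or falling) and sets the flipbook only when it changes.
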(event `self.ReceiveBeginPlay`
  (bind _asgm_ctrl_alt_24 (cast `/Game/CtrlAltJam/Blueprints/Core/GM_CtrlAlt24` (`GameplayStatics.GetGameMode`)))
  (set `self.GameMode` _asgm_ctrl_alt_24)
  (add `/Game/CtrlAltJam/Blueprints/Core/GM_CtrlAlt24.OnImpulseAdded` (`self.GameMode`) (`|CreateDelegate` :!event `OnImpulseAdded_Event`)))

(event `OnImpulseAdded_Event`
  (params (ScenarioImpulse :type "Float (double-precision)") (CharacterImpulse :type "Float (double-precision)"))
  (if (> CharacterImpulse 0.0)
    (`/Engine/EditorBlueprintResources/StandardMacros.DoOnce` false
      (:`Completed`
        (set `self.LeftGroundAtLeastOnce` true)
        (remove `/Game/CtrlAltJam/Blueprints/Core/GM_CtrlAlt24.OnImpulseAdded` (`self.GameMode`) (`|CreateDelegate` :!event `OnImpulseAdded_Event`))))))

(event `self.ReceiveTick`
  (params (DeltaSeconds :type "Float (single-precision)"))
  (bind (_returnvalue_x _returnvalue_y _returnvalue_z) (`KismetMathLibrary.BreakVector` (`self.GetVelocity`)))
  (bind _returnvalue (select `bool` (`KismetMathLibrary.NearlyEqual_FloatFloat` _returnvalue_z 0.0 0.1) :`false` (select `bool` (< _returnvalue_z 0.0) :`false` "/Game/CtrlAltJam/Materials/Du/Jump/FB_DuJump.FB_DuJump" :`true` "/Game/CtrlAltJam/Materials/Du/Fly/FB_DuFly.FB_DuFly" :!type "PaperFlipbook Object Reference") :`true` "/Game/CtrlAltJam/Materials/Du/Idle/FB_DuIdle.FB_DuIdle"))
  (`|ExecutionSequence`
    (:`then_1`
      (if (`self.LeftGroundAtLeastOnce`)
        (if (!= _returnvalue (`self.CurrentFlipbook`))
          (bind _output_get (set `self.CurrentFlipbook` _returnvalue))
          (`PaperFlipbookComponent.SetFlipbook` (`self.FB_Du`) _output_get))))))

(fn `UserConstructionScript`)