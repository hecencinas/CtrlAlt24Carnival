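; Game mode that runs a scrolling backdrop of pooled BP_DefaultHomeSetup actors along the Y axis.
; On BeginPlay it spawns a row between tagged start and finish points, plus extra off-screen pieces.
; AddScenarioImpulse sets their physics velocity.
; Tick accumulates impulse over time, not checking positions, to periodically teleport the next piece, round-robin, to the renew position at the row's end.
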(event `self.ReceiveBeginPlay`
  (`parent.ReceiveBeginPlay`)
  (`|ExecutionSequence`
    (:`then_0`
      (bind _outactors (`GameplayStatics.GetAllActorsWithTag` "StartingPoint"))
      (if (`KismetArrayLibrary.Array_IsNotEmpty` _outactors)
        (set `self.StartingPoint` (`|GetArrayItem` _outactors))))
    (:`then_1`
      (bind _outactors_2 (`GameplayStatics.GetAllActorsWithTag` "FinishingPoint"))
      (if (`KismetArrayLibrary.Array_IsNotEmpty` _outactors_2)
        (set `self.FinishingPoint` (`|GetArrayItem` _outactors_2))))
    (:`then_2`
      (`self.SpawnScenario`))))

(event `AddScenarioImpulse`
  (set `self.ScenarioImpulse` 10.0)
  (for _array_element (`self.SpawnedScenarios`)
    (`/Engine/EditorBlueprintResources/StandardMacros.IsValid` _array_element
      (:`Is Valid`
        (`PrimitiveComponent.SetPhysicsLinearVelocity` (cast `PrimitiveComponent` (`Actor.RootComponent` _array_element) :!pure true) (`KismetMathLibrary.MakeVector` 0.0 (* (`self.ScenarioImpulse`) (`self.ScenarioBaseImpulse`))) false "None")))))

(event `self.ReceiveTick`
  (params (DeltaSeconds :type "Float (single-precision)"))
  (bind _scenarioimpulse (`self.ScenarioImpulse`))
  (if (> _scenarioimpulse 0.0)
    (set `self.PoolRenewDelta` (+ (`self.PoolRenewDelta`) (/ (* _scenarioimpulse DeltaSeconds) 15.0)))
    (if (> (`self.PoolRenewDelta`) 1.0)
      (set `self.PoolRenewDelta` 0.0)
      (`self.K2_SetActorLocation` (`|GetArrayItem` (`self.SpawnedScenarios`) (`self.LastRenewedIndex`)) (`self.RenewPosition`) false true)
      (bind _result (`/Engine/EditorBlueprintResources/StandardMacros.IncrementInt` (`self.LastRenewedIndex`))
        (:`  `
          (if (== _result (`KismetArrayLibrary.Array_Length` (`self.SpawnedScenarios`)))
            (set `self.LastRenewedIndex` 0)))))))

(fn `SpawnScenario`
  (bind (_returnvalue_x _returnvalue_y) (`KismetMathLibrary.BreakVector` (`self.K2_GetActorLocation` (`self.FinishingPoint`))))
  (bind (_returnvalue_x_2 _returnvalue_y_2) (`KismetMathLibrary.BreakVector` (`self.K2_GetActorLocation` (`self.FinishingPoint`))))
  (bind (_returnvalue_x_3 _returnvalue_y_3) (`KismetMathLibrary.BreakVector` (`self.K2_GetActorLocation` (`self.FinishingPoint`))))
  (bind (_returnvalue_x_4 _returnvalue_y_4) (`KismetMathLibrary.BreakVector` (`self.K2_GetActorLocation` (`self.StartingPoint`))))
  (bind _returnvalue (`self.GetTransform` (`self.StartingPoint`)))
  (bind _returnvalue_2 (`KismetMathLibrary.FTrunc` (/ (- _returnvalue_y_4 _returnvalue_y) (`self.ScenarioWidth`))))
  (for _index (range (+ (+ (`self.ExtraNonVisiblePoolToSpawn`) _returnvalue_2) 1))
    (bind _returnvalue_3 (`|SpawnActorFromClass` "/Game/CtrlAltJam/Blueprints/BP_DefaultHomeSetup.BP_DefaultHomeSetup_C" (`KismetMathLibrary.MakeTransform` (`KismetMathLibrary.MakeVector` (.x (.location _returnvalue)) (+ (* _index (`self.ScenarioWidth`)) _returnvalue_y_3) (.z (.location _returnvalue))) (.rotation _returnvalue) (.scale _returnvalue)) "Undefined" "MultiplyWithRoot" null null))
    (`KismetArrayLibrary.Array_Add` (`self.SpawnedScenarios`) _returnvalue_3))
  (set `self.RenewPosition` (`KismetMathLibrary.MakeVector` (.x (.location _returnvalue)) (+ (* (+ _returnvalue_2 (`self.ExtraNonVisiblePoolToSpawn`)) (`self.ScenarioWidth`)) _returnvalue_y_2) (.z (.location _returnvalue)))))

(fn `UserConstructionScript`)