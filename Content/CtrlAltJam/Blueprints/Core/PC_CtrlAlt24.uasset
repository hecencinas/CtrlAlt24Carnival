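; PC_CtrlAlt24 is a player controller that adds a debug Z key to launch the main character upward.
; On BeginPlay it caches the first BP_MainCharacter in the level and the GM_CtrlAlt24 game mode.
; The key press applies a vertical impulse to the character's Sphere and calls AddScenarioImpulse on the game mode.
; A DoOnce reset after a short delay acts as the cooldown between presses.
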(event EventBeginPlay
  (bind _outactors (Actor|GetAllActorsOfClass "/Game/CtrlAltJam/Blueprints/Core/BP_MainCharacter.BP_MainCharacter_C"))
  (if (Utilities|Array|IsNotEmpty _outactors)
    (Variables|Default|SetMainCharacter (Utilities|Array|Get(acopy) _outactors))
    (bind _asgm_ctrl_alt_24 (Utilities|Casting|CastToGM_CtrlAlt24 (Game|GetGameMode)))
    (Variables|Default|SetGameMode _asgm_ctrl_alt_24)))

(event Input|KeyboardEvents|DebugKeyZ
  (params (Key :type Key%20Structure :default "None") (ActionValue :type Input%20Action%20Value%20Structure))
  (:Pressed
    (Utilities|FlowControl|DoOnce false :!label _label
      (:Completed
        (Physics|AddImpulse (Variables|/Game/CtrlAltJam/Blueprints/Core/BP_MainCharacter.BP_MainCharacter_C|GetSphere (Variables|Default|GetMainCharacter)) "0.000000,0.000000,10000.000000" "None" false)
        (Default|AddScenarioImpulse (Variables|Default|GetGameMode))
        (Utilities|FlowControl|Delay 1.5)
        (goto _label Reset)))))

(fn ConstructionScript)